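; BP_P38 is a player-flown P-38 plane that constantly moves forward, steers and fires rockets.
; Tick feeds the player pawn's forward vector and MaxScale into movement input and spins both propellers through RotateFunction.
; Pitch and Roll axes apply clamped, frame-rate-independent local rotations, while Boost raises MaxScale only while held.
; Pressing Fire spawns a BP_Rocket at the Arrow component's transform.
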(event EventTick
  (params (DeltaSeconds :type Float%20%28single-precision%29))
  ;[1 1 1] Add Movement Input , RotatePropeler
  (Pawn|Input|AddMovementInput (Transformation|GetActorForwardVector (Game|Player|GetPlayerPawn 0)) (Variables|Default|GetMaxScale) false)
  (CallFunction|RotateFunction (Variables|Default|GetRightPropeler))
  (CallFunction|RotateFunction (Variables|Default|GetLeftPropeler)))

(event Input|ActionEvents|InputActionFire
  (params (Key :type Key%20Structure :default "None"))
  ;[1 1 1] Fire
  (:Pressed
    (Game|SpawnActorfromClass "/Game/Blueprints/BP_Rocket.BP_Rocket_C" (Transformation|GetWorldTransform (Variables|Default|GetArrow)) "Undefined" "MultiplyWithRoot" 0 0)))

(event Input|ActionEvents|InputActionBoost
  (params (Key :type Key%20Structure :default "None"))
  ;[1 1 1] Boost
  (:Pressed
    (Variables|Default|SetMaxScale 1.0))
  (:Released
    (Variables|Default|SetMaxScale 0.2)))

(event Input|AxisEvents|InputAxisPitch
  (params (AxisValue :type Float%20%28single-precision%29))
  ;[1 1 1] Pitch
  (Transformation|AddActorLocalRotation (Math|Rotator|MakeRotator 0.0 (* (Math|Float|Clamp(Float) AxisValue -1.0) 6e+01 (Utilities|Time|GetWorldDeltaSeconds)) 0.0) false false))

(event Input|AxisEvents|InputAxisRoll
  (params (AxisValue :type Float%20%28single-precision%29))
  ;[1 1 1] Roll
  (Transformation|AddActorLocalRotation (Math|Rotator|MakeRotator (* (Math|Float|Clamp(Float) AxisValue -1.0) 6e+01 (Utilities|Time|GetWorldDeltaSeconds)) 0.0 0.0) false false))

(fn ConstructionScript)

(fn RotateFunction
  (params (self2 :type Scene%20Component%20Object%20Reference))
  (Transformation|AddRelativeRotation self2 (Math|Rotator|MakeRotator (* (Utilities|Time|GetWorldDeltaSeconds) 3.6e+03) 0.0 0.0) false false)
  (return))